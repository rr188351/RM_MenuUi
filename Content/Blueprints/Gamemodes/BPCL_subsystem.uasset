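; Settings subsystem that persists and serves the player's audio and gameplay options through an SG_UserSettings save object.
; LoadSettings lazily returns the cached object, else loads it from the slot or creates one.
; Getters expose volume, difficulty, mouse options and gameplay defaults, while save functions replace a settings struct and write to disk.
; The async load event only reloads when a cached object is already valid.
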(event Custom|asyn%20load
  (params (WorldContextObject :type Object%20Object%20Reference))
  (bind _settingssaveslott (Variables|Default|GetSettingsSaveSlott))
  (Variables|Default|GetSG_UserSettings
    (:then
      (bind _returnvalue (SaveGame|DoesSaveGameExist _settingssaveslott))
      (if _returnvalue
        (bind _savegame (|AsyncLoadGamefromSlot WorldContextObject _settingssaveslott)
          (:then
            (bind _assg_user_settings (Utilities|Casting|CastToSG_UserSettings _savegame))
            (Variables|Default|SetSG_UserSettings _assg_user_settings)))))
    (:else)))

(fn SaveAudioSettings
  (params (AudioSettings :type S%20Audio%20Settings%20Structure))
  (Variables|/RM_MenuUI/Blueprints/saveGame/SG_UserSettings.SG_UserSettings_C|SetAudioSettings (CallFunction|LoadSettings) AudioSettings)
  (CallFunction|SaveSettings))

(fn LoadSettings
  (bind _settingssaveslott (Variables|Default|GetSettingsSaveSlott))
  (Variables|Default|GetSG_UserSettings
    (:then
      _)
    (:else
      (bind _returnvalue (SaveGame|DoesSaveGameExist _settingssaveslott))
      (if _returnvalue
        (bind _returnvalue_2 (SaveGame|LoadGamefromSlot _settingssaveslott))
        (bind _assg_user_settings (Utilities|Casting|CastToSG_UserSettings _returnvalue_2))
        (Variables|Default|SetSG_UserSettings _assg_user_settings)
        (else
          (bind _returnvalue_3 (SaveGame|CreateSaveGameObject "/RM_MenuUI/Blueprints/saveGame/SG_UserSettings.SG_UserSettings_C"))
          (Variables|Default|SetSG_UserSettings _returnvalue_3)))))
  (return (Variables|Default|GetSG_UserSettings)))

(fn SaveSettings
  (bind _returnvalue (SaveGame|SaveGametoSlot (Variables|Default|GetSG_UserSettings) (Variables|Default|GetSettingsSaveSlott)))
  (Development|PrintString 0 (Utilities|String|Append "Setting Saved" (Utilities|String|ToString(Boolean) _returnvalue)) true true "(R=0.000000,G=0.660000,B=1.000000,A=1.000000)" 5.0))

(fn GetSA
  (bind _sg_usersetting (CallFunction|LoadSettings))
  (Utilities|IsValid _sg_usersetting
    (:Is%20Valid
      (return (Utilities|Struct|BreakS_AudioSettings (Variables|/RM_MenuUI/Blueprints/saveGame/SG_UserSettings.SG_UserSettings_C|GetAudioSettings _sg_usersetting))))))

(fn GetDifficulty
  (return (Variables|Default|GetDifficultyPresents) (Utilities|Struct|BreakS_Gameplaysettings (Variables|/RM_MenuUI/Blueprints/saveGame/SG_UserSettings.SG_UserSettings_C|GetGameplaySett (CallFunction|LoadSettings)))))

(fn IsMouseYinvert
  (return (Utilities|Struct|BreakS_Gameplaysettings (Variables|/RM_MenuUI/Blueprints/saveGame/SG_UserSettings.SG_UserSettings_C|GetGameplaySett (CallFunction|LoadSettings)))))

(fn GetMouseSensivity
  (return 0.1 1.0 (Utilities|Struct|BreakS_Gameplaysettings (Variables|/RM_MenuUI/Blueprints/saveGame/SG_UserSettings.SG_UserSettings_C|GetGameplaySett (CallFunction|LoadSettings)))))

(fn SaveGameplaySett
  (params (GameplaySettings :type S%20Gameplaysettings%20Structure))
  (Variables|/RM_MenuUI/Blueprints/saveGame/SG_UserSettings.SG_UserSettings_C|SetGameplaySett (CallFunction|LoadSettings) GameplaySettings)
  (CallFunction|SaveSettings))

(fn GetDefaultGameplaySettings
  (return (Variables|Default|GetDefaultsgame)))